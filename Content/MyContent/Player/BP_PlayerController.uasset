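; Player controller that routes Enhanced Input to the possessed BP_PlayerCharacter and owns the player's HUD and game menu.
; On possess it caches the character, adds camera, jump, movement and combat mapping contexts, shows the HUD and creates the game menu hidden.
; Input actions forward sensitivity-scaled camera, movement, jump and basic combo attack to the character, while a toggle action adds or removes the menu.
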(event Input|EnhancedActionEvents|EnhancedInputActionIA_Jump
  (params (ActionValue :type Boolean) (ElapsedSeconds :type Float%20%28double-precision%29) (TriggeredSeconds :type Float%20%28double-precision%29) (InputAction :type Input%20Action%20Object%20Reference :default "/Game/MyContent/Player/Input/IA_Jump.IA_Jump"))
  (Default|TryJump (Variables|Default|GetCharRef) ActionValue))

(event Input|EnhancedActionEvents|EnhancedInputActionIA_Camera
  (params (ActionValue :type Vector%202D%20Structure) (ElapsedSeconds :type Float%20%28double-precision%29) (TriggeredSeconds :type Float%20%28double-precision%29) (InputAction :type Input%20Action%20Object%20Reference :default "/Game/MyContent/Player/Input/IA_Camera.IA_Camera"))
  (Default|ControlCamera (Variables|Default|GetCharRef) (* ActionValue (Variables|Default|GetCameraSensitivity))))

(event Input|EnhancedActionEvents|EnhancedInputActionIA_Move
  (params (ActionValue :type Vector%202D%20Structure) (ElapsedSeconds :type Float%20%28double-precision%29) (TriggeredSeconds :type Float%20%28double-precision%29) (InputAction :type Input%20Action%20Object%20Reference :default "/Game/MyContent/Player/Input/IA_Move.IA_Move"))
  (:Triggered
    (Default|MoveCharacter (Variables|Default|GetCharRef) ActionValue :!label _label))
  (:Started
    (goto _label))
  (:Canceled
    (goto _label))
  (:Completed
    (goto _label)))

(event Input|EnhancedActionEvents|EnhancedInputActionIA_BasicAttack
  (params (ActionValue :type Boolean) (ElapsedSeconds :type Float%20%28double-precision%29) (TriggeredSeconds :type Float%20%28double-precision%29) (InputAction :type Input%20Action%20Object%20Reference :default "/Game/MyContent/Player/Input/IA_BasicAttack.IA_BasicAttack"))
  (Default|BasicComboAttack (Variables|Default|GetCharRef)))

(event Input|EnhancedActionEvents|EnhancedInputActionIA_ToggleGameMenu
  (params (ActionValue :type Boolean) (ElapsedSeconds :type Float%20%28double-precision%29) (TriggeredSeconds :type Float%20%28double-precision%29) (InputAction :type Input%20Action%20Object%20Reference :default "/Game/MyContent/Player/Input/IA_ToggleGameMenu.IA_ToggleGameMenu"))
  (CallFunction|ToggleGameMenu))

(event EventPossess
  (params (PossessedPawn :type Pawn%20Object%20Reference))
  (bind _asbp_player_character (Utilities|Casting|CastToBP_PlayerCharacter PossessedPawn))
  (Variables|Default|SetCharRef _asbp_player_character)
  (CallFunction|SetDefaultInputs)
  (bind _returnvalue (UserInterface|CreateWidget "/Game/MyContent/Player/HUD/BP_UI_Player_HUD.BP_UI_Player_HUD_C"))
  (bind _output_get (Variables|Default|SetPlayerHUD _returnvalue))
  (UserInterface|Viewport|AddtoPlayerScreen _output_get)
  (bind _returnvalue_2 (UserInterface|CreateWidget "/Game/MyContent/Player/GameMenu/BP_UI_GameMenu.BP_UI_GameMenu_C"))
  (Variables|Default|SetGameMenu _returnvalue_2))

(fn ConstructionScript)

(fn AddInput
  (params (MappingContext :type Input%20Mapping%20Context%20Object%20Reference) (Priority :type Integer) (%20Ignore%20All%20Pressed%20Keys%20Until%20Release :type Boolean))
  (Input|AddMappingContext (PlayerController|LocalPlayerSubsystems|GetEnhancedInputLocalPlayerSubsystem) MappingContext Priority (Utilities|Struct|MakeModifyContextOptions %20Ignore%20All%20Pressed%20Keys%20Until%20Release false false)))

(fn SetDefaultInputs
  (for _array_element (Utilities|Array|MakeArray "/Game/MyContent/Player/Input/IMC_Camera.IMC_Camera" "/Game/MyContent/Player/Input/IMC_Jump.IMC_Jump" "/Game/MyContent/Player/Input/IMC_Movement.IMC_Movement" "/Game/MyContent/Player/Input/IMC_Combat.IMC_Combat")
    (CallFunction|AddInput _array_element 0 true)))

(fn RemoveInput
  (params (MappingContext :type Input%20Mapping%20Context%20Object%20Reference) (Ignore%20All%20Pressed%20Keys%20Until%20Release :type Boolean))
  (Input|RemoveMappingContext (PlayerController|LocalPlayerSubsystems|GetEnhancedInputLocalPlayerSubsystem) MappingContext (Utilities|Struct|MakeModifyContextOptions Ignore%20All%20Pressed%20Keys%20Until%20Release false false)))

(fn ToggleGameMenu
  (bind _gamemenu (Variables|Default|GetGameMenu))
  (if (not (UserInterface|Viewport|IsinViewport (Variables|Default|GetGameMenu)))
    (UserInterface|Viewport|AddtoPlayerScreen _gamemenu)
    (else
      (Widget|RemovefromParent _gamemenu))))