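; BP_Weapon is a weapon item that deals damage to actors overlapping its DamageCollider.
; ActivateDamage and DeactivateDamage switch the collider between query-only and no collision, opening and closing the damage window.
; On overlap it applies Damage with its owner as causer, skipping the owner and any actor whose class derives from an entry in ClassesToIgnore.
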(event OnComponentBeginOverlap(DamageCollider)
  (params (OverlappedComponent :type Primitive%20Component%20Object%20Reference) (OtherActor :type Actor%20Object%20Reference) (OtherComp :type Primitive%20Component%20Object%20Reference) (OtherBodyIndex :type Integer) (bFromSweep :type Boolean) (SweepResult :type Hit%20Result%20Structure%20%28by%20ref%29))
  (if (and (not (CallFunction|IsIgnoredClass OtherActor)) (!= OtherActor (Components|GetOwner)))
    (Game|Damage|ApplyDamage OtherActor (Variables|Weapon|GetDamage) 0 (Components|GetOwner))))

(fn ConstructionScript)

(fn ActivateDamage
  (Collision|SetCollisionEnabled (Variables|Default|GetDamageCollider) "QueryOnly"))

(fn DeactivateDamage
  (Collision|SetCollisionEnabled (Variables|Default|GetDamageCollider) "NoCollision"))

(fn IsIgnoredClass
  (params (TestActor :type Actor%20Object%20Reference))
  (for _array_element (Variables|Weapon|GetClassesToIgnore)
    (if (Utilities|ClassIsChildOf (Utilities|GetClass TestActor) _array_element)
      (return true)))
  (return false))