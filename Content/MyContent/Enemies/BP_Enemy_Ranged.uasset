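; BP_Enemy_Ranged is a ranged enemy that deals damage by firing a projectile at its target.
; ActivateDamage spawns ProjectileClass at ProjectileSpawnLocation, owned by the enemy and given the TargetActor.
; Only the pitch is aimed at the target through a look-at rotation, while yaw and roll follow the spawn component.
; The event graph and construction script add no logic of their own.
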(event EventBeginPlay
  (|CallParentFunction) ; This node is disabled and will not be called.\nDrag off pins to build functionality.
)

(event Collision|EventActorBeginOverlap
  (params (OtherActor :type Actor%20Object%20Reference)))

(event EventTick
  (params (DeltaSeconds :type Float%20%28single-precision%29)))

(fn ConstructionScript
  (|CallParentFunction))

(fn ActivateDamage
  (bind _projectilespawnlocation (Variables|Default|GetProjectileSpawnLocation))
  (bind _returnvalue (Transformation|GetWorldRotation _projectilespawnlocation))
  (Game|SpawnActorfromClass (Variables|Default|GetProjectileClass) (Math|Transform|MakeTransform (Transformation|GetWorldLocation _projectilespawnlocation) (Math|Rotator|MakeRotator (.roll _returnvalue) (.pitch (Math|Rotator|FindLookatRotation (Transformation|GetWorldLocation (Variables|Default|GetProjectileSpawnLocation)) (Transformation|GetActorLocation (Variables|Default|GetTargetActor)))) (.yaw _returnvalue)) "1.000000,1.000000,1.000000") "Undefined" "MultiplyWithRoot" self (Variables|Default|GetTargetActor) 1.0 false 0))