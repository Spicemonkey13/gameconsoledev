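; BP_EnemyController is the AI controller for enemy characters, driving each pawn's own behavior tree.
; On possession it runs the enemy's Behaviour tree and copies its AttackRange into the blackboard.
; Perception locks onto the first perceived player character while no valid target is held, updating both blackboard and enemy.
; InterruptAI writes a duration to the InterruptTime blackboard key.
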(event OnTargetPerceptionUpdated(AIPerception)
  (params (Actor :type Actor%20Object%20Reference) (Stimulus :type AI%20Stimulus%20Structure))
  (if (not (Utilities|IsValid (Variables|Default|GetTargetActor)))
    (bind _asbp_player_character (Utilities|Casting|CastToBP_PlayerCharacter Actor))
    (CallFunction|SetControlTarget _asbp_player_character)))

(event EventPossess
  (params (PossessedPawn :type Pawn%20Object%20Reference))
  (bind _asbp_enemy_character (Utilities|Casting|CastToBP_EnemyCharacter PossessedPawn))
  (bind _output_get (Variables|Default|SetEnemyRef _asbp_enemy_character))
  (bind _behaviour (Variables|/Game/MyContent/Enemies/BP_EnemyCharacter.BP_EnemyCharacter_C|GetBehaviour _output_get)
    (:then
      (AI|RunBehaviorTree _behaviour)
      (CallFunction|SetDefaultBBKeys))
    (:else)))

(fn ConstructionScript)

(fn SetControlTarget
  (params (TargetActor :type Actor%20Object%20Reference))
  (bind _output_get (Variables|Default|SetTargetActor TargetActor))
  (AI|Components|Blackboard|SetValueasObject (AI|GetBlackboard 0) (Utilities|Name|MakeLiteralName "TargetActor") _output_get)
  (Default|SetEnemyTarget (Variables|Default|GetEnemyRef) (Variables|Default|GetTargetActor)))

(fn InterruptAI
  (params (Duration :type Float%20%28double-precision%29))
  (AI|Components|Blackboard|SetValueasFloat (AI|GetBlackboard 0) (Utilities|Name|MakeLiteralName "InterruptTime") Duration))

(fn SetDefaultBBKeys
  (AI|Components|Blackboard|SetValueasFloat (AI|GetBlackboard 0) (Utilities|Name|MakeLiteralName "AttackRange") (Variables|/Game/MyContent/Enemies/BP_EnemyCharacter.BP_EnemyCharacter_C|GetAttackRange (Variables|Default|GetEnemyRef))))