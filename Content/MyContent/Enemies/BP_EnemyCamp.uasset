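; BP_EnemyCamp is an enemy camp actor that keeps a list of member enemies, intended for group alerts.
; AddEnemy and RemoveEnemy maintain that list.
; AlertCamp sets a one-time alerted flag, then loops over the members, checking for those other than the enemy that raised the alert.
; The SetAITarget call that would pass the target to those members is disconnected, so alerts currently do not propagate.
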(event EventBeginPlay)

(event Collision|EventActorBeginOverlap
  (params (OtherActor :type Actor%20Object%20Reference)))

(event EventTick
  (params (DeltaSeconds :type Float%20%28single-precision%29)))

(fn ConstructionScript)

(fn AddEnemy
  (params (Enemy :type BP%20Enemy%20Character%20Object%20Reference%20%28by%20ref%29))
  (Utilities|Array|Add (Variables|Default|GetEnemiesInCamp) Enemy))

(fn RemoveEnemy
  (params (Enemy :type BP%20Enemy%20Character%20Object%20Reference%20%28by%20ref%29))
  (Utilities|Array|RemoveItem (Variables|Default|GetEnemiesInCamp) Enemy))

(fn AlertCamp
  (params (AlertedEnemy :type BP%20Enemy%20Character%20Object%20Reference) (Target :type Actor%20Object%20Reference))
  (if (not (Variables|Default|GetbCampAlerted))
    (Variables|Default|SetbCampAlerted true)
    (for _array_element (Variables|Default|GetEnemiesInCamp)
      (if (!= _array_element AlertedEnemy)
        _))))