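; Player stats actor component that tracks experience and handles leveling up.
; XP and MaxXP setters clamp values to zero or above and fire an XP change notification.
; AddXP raises XP, signals the gain and calls LevelUp once when XP reaches MaxXP.
; LevelUp increments Level, carries surplus XP over by subtracting MaxXP, then signals the level-up.
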(fn SetXP
  (params (XP :type Float%20%28double-precision%29))
  (Variables|Default|SetXP (Math|Float|Max(Float) XP 0.0))
  (Default|CallOnXPChange))

(fn SetMaxXP
  (params (MaxXP :type Float%20%28double-precision%29))
  (Variables|Default|SetMaxXP (Math|Float|Max(Float) MaxXP 0.0))
  (Default|CallOnXPChange))

(fn AddXP
  (params (Amount :type Float%20%28double-precision%29))
  (CallFunction|SetXP (+ (Variables|Default|GetXP) Amount))
  (Default|CallOnXPAdded Amount)
  (if (>= (Variables|Default|GetXP) (Variables|Default|GetMaxXP))
    (CallFunction|LevelUp)))

(fn LevelUp
  (CallFunction|SetLevel (+ (Variables|Default|GetLevel) 1.0))
  (CallFunction|SetXP (- (Variables|Default|GetXP) (Variables|Default|GetMaxXP)))
  (Default|CallOnLevelUp))