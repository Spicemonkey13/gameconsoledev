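; BP_AC_Stats is a stats component that tracks Health, MaxHealth and Level for its owner.
; Damage and heal functions route through SetHealth, which clamps between zero and MaxHealth, then fire their own Damaged or Healed events.
; Setters broadcast health or level change events, and IsAlive reports whether Health is above zero.
; SetMaxHealth only floors the maximum at zero and does not re-clamp current Health.
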(fn SetHealth
  (params (NewParam :type Float%20%28double-precision%29))
  (Variables|Default|SetHealth (Math|Float|Clamp(Float) NewParam 0.0 (Variables|Default|GetMaxHealth)))
  (Default|CallOnHealthChanged))

(fn SetMaxHealth
  (params (MaxHealth :type Float%20%28double-precision%29))
  (Variables|Default|SetMaxHealth (Math|Float|Max(Float) MaxHealth 0.0))
  (Default|CallOnHealthChanged))

(fn DamageHealth
  (params (Amount :type Float%20%28double-precision%29))
  (CallFunction|SetHealth (- (Variables|Default|GetHealth) Amount))
  (Default|CallOnDamaged Amount))

(fn HealHealth
  (params (Amount :type Float%20%28double-precision%29))
  (CallFunction|SetHealth (+ (Variables|Default|GetHealth) Amount))
  (Default|CallOnHealed))

(fn SetLevel
  (params (Level :type Float%20%28double-precision%29))
  (Variables|Default|SetLevel Level)
  (Default|CallOnLevelChanged))

(fn IsAlive
  (return (> (Variables|Default|GetHealth) 0.0)))