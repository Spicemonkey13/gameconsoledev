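; BP_Projectile is a projectile that damages actors it overlaps and is destroyed on contact.
; Overlaps on its DamageCollison component ignore the owner, and apply damage only to TargetActor unless CanDamageAnything is set, with the owner as damage causer.
; Any non-owner overlap then calls OnHit, a separate function that destroys the projectile, even when no damage was dealt.
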(event OnComponentBeginOverlap(DamageCollison)
  (params (OverlappedComponent :type Primitive%20Component%20Object%20Reference) (OtherActor :type Actor%20Object%20Reference) (OtherComp :type Primitive%20Component%20Object%20Reference) (OtherBodyIndex :type Integer) (bFromSweep :type Boolean) (SweepResult :type Hit%20Result%20Structure%20%28by%20ref%29))
  (Variables|Default|SetHitActor OtherActor)
  (if (!= OtherActor (Components|GetOwner))
    (Utilities|FlowControl|Sequence
      (:then_0
        (if (or (== OtherActor (Variables|Default|GetTargetActor)) (Variables|Default|GetbCanDamageAnything))
          (Game|Damage|ApplyDamage (Variables|Default|GetHitActor) (Variables|Default|GetDamage) 0 (Components|GetOwner))))
      (:then_1
        (CallFunction|OnHit)))))

(fn ConstructionScript)

(fn OnHit
  (Actor|DestroyActor))